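; Enemy spawn point that spawns one random zombie for the current wave of the BP_TurnBased game mode.
; SpawnEnemy reads the wave's DT_WaveData row and expands its EnemyPool counts into the Zombies array as a weighted pool, never cleared between calls.
; It spawns a random pick at its own X, Y and rotation with a fixed height, then sets itself as the zombie's Spawner.
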(event Custom|SpawnEnemy
  (bind _returnvalue (Transformation|GetActorTransform))
  (bind _zombies (Variables|Default|GetZombies))
  (bind _returnvalue_2 (Utilities|GetDataTableRow "/Game/BluePrints/DT_WaveData.DT_WaveData" (Utilities|String|StringToName (Utilities|String|ToString(Integer) (Variables|/Game/BluePrints/BP_TurnBased.BP_TurnBased_C|GetCurrentWave (Variables|Default|GetAs%20BP%20Turn%20Based)))))
    (:then
      (bind _keys (Utilities|Map|Keys (.EnemyPool (Utilities|Struct|BreakEnemyPool1 _returnvalue_2))))
      (for _array_element _keys
        (for _index (range 1 (.Value (Utilities|Map|Find (.EnemyPool (Utilities|Struct|BreakEnemyPool1 _returnvalue_2)) _array_element)))
          (Utilities|Array|Add (Variables|Default|GetZombies) _array_element)))
      (bind _output_get (Variables|Default|SetZombieToSpawn (Utilities|Array|Get(acopy) _zombies (Math|Random|RandomIntegerinRange 0 (Utilities|Array|LastIndex _zombies)))))
      (Development|PrintString (Utilities|GetClassDisplayName _output_get))
      (bind _returnvalue_3 (Game|SpawnActorfromClass _output_get (Math|Transform|MakeTransform (Math|Vector|MakeVector (.x (.location _returnvalue)) (.y (.location _returnvalue)) 291.0) (.rotation _returnvalue) "1.000000,1.000000,1.000000") "AdjustIfPossibleButAlwaysSpawn" "OverrideRootScale" 0 0))
      (Variables|/Game/BluePrints/BP_Zombie.BP_Zombie_C|SetSpawner _returnvalue_3 self))))

(event EventBeginPlay
  (bind _asbp_turn_based (Utilities|Casting|CastToBP_TurnBased (Game|GetGameMode)))
  (Variables|Default|SetAs%20BP%20Turn%20Based _asbp_turn_based))

(event Collision|EventActorBeginOverlap
  (params (OtherActor :type Actor%20Object%20Reference)))

(event EventTick
  (params (DeltaSeconds :type Float%20%28single-precision%29)))

(fn ConstructionScript)