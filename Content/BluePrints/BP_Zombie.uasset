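; BP_Zombie is a turn-based enemy character that chases the player and shows its HP on an InspectText widget.
; On StartTurn it walks toward the player through its AI controller for a fixed time, stops, then ends the turn on the BP_TurnBased game mode.
; TakeDamage lowers Health and refreshes the widget, and at zero removes the zombie from the game mode's OutActors before destroying it.
; No attack logic is wired.
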(event EventBeginPlay
  (Physics|SetSimulatePhysics (Variables|Character|GetMesh) false)
  (Utilities|FlowControl|Delay 0.1)
  (bind _asinspect_text (Utilities|Casting|CastToInspectText (UserInterface|GetWidget (Variables|Default|GetWidget))))
  (Default|UpdateInspectText _asinspect_text (Utilities|Text|ToText(String) (Utilities|String|Append "HP:" (Utilities|String|ToString(Integer) (Variables|Default|GetHealth)))))
  (Appearance|SetColorandOpacity _asinspect_text "(R=0.000000,G=1.000000,B=0.739300,A=1.000000)" :!class /Script/UMG.UserWidget))

(event Collision|EventActorBeginOverlap
  (params (OtherActor :type Actor%20Object%20Reference)))

(event EventTick
  (params (DeltaSeconds :type Float%20%28single-precision%29)))

(event EventEndTurn)

(event EventStartTurn
  (bind _asbp_player (Utilities|Casting|CastToBP_Player (Game|GetPlayerCharacter 0)))
  (AI|Navigation|SimpleMovetoLocation (AI|GetAIController self) (.location (Transformation|GetActorTransform _asbp_player)))
  (Utilities|FlowControl|Delay 2.0)
  (Components|Movement|StopMovementImmediately (Variables|Character|GetCharacterMovement))
  (bind _asbp_turn_based (Utilities|Casting|CastToBP_TurnBased (Game|GetGameMode)))
  (Utilities|FlowControl|Delay 1.0)
  (Default|EndTurn _asbp_turn_based))

(event EventTakeDamage
  (params (DamageAmount :type Integer))
  (bind _output_get (Variables|Default|SetHealth (- (Variables|Default|GetHealth) DamageAmount)))
  (bind _asinspect_text (Utilities|Casting|CastToInspectText (UserInterface|GetWidget (Variables|Default|GetWidget))))
  (Default|UpdateInspectText _asinspect_text (Utilities|Text|ToText(String) (Utilities|String|Append "HP:" (Utilities|String|ToString(Integer) (Variables|Default|GetHealth)))))
  (if (<= _output_get 0)
    (Utilities|FlowControl|Delay 1.0)
    (bind _asbp_turn_based (Utilities|Casting|CastToBP_TurnBased (Game|GetGameMode)))
    (Utilities|Array|RemoveItem (Variables|/Game/BluePrints/BP_TurnBased.BP_TurnBased_C|GetOut%20Actors _asbp_turn_based) self)
    (Actor|DestroyActor)))

(fn ConstructionScript)

(fn NewFunction)