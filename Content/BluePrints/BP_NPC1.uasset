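; BP_NPC1 is a clickable NPC offering branching dialogue and a temporary floating inspect text.
; Interact binds Talk to the HUD context menu; Talk walks the player over and arms a sphere whose overlap pauses the player, blends the camera and opens dialogue.
; DataTable rows chain the lines: clicks advance or end the conversation and restore control, while open-ended rows spawn WB_Option choices that feed OptionSelected.
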(event Custom|Talk
  (bind _asbp_player (Utilities|Casting|CastToBP_Player (Game|GetPlayerCharacter 0)))
  (AI|Navigation|SimpleMovetoLocation (Game|GetPlayerController 0) (Transformation|GetActorLocation (Variables|/Game/BluePrints/BP_Player.BP_Player_C|GetHit%20Actor _asbp_player)))
  (bind _asbp_player_2 (Utilities|Casting|CastToBP_Player (Game|GetPlayerCharacter 0)))
  (bind _asbp_npc1 (Utilities|Casting|CastToBP_NPC1 (Variables|/Game/BluePrints/BP_Player.BP_Player_C|GetHit%20Actor _asbp_player_2)))
  (Components|Activation|Activate (Variables|BP_NPC1_C|GetSphere _asbp_npc1) false)
  (Variables|/Script/Engine.PrimitiveComponent|SetbGenerateOverlapEvents (Variables|Default|GetSphere) true))

(event Custom|MouseClicked
  (bind _returnvalue (Game|GetPlayerController 0))
  (bind _sphere (Variables|Default|GetSphere))
  (if (Variables|Default|GetEndDialogue)
    (Widget|RemovefromParent (Variables|Default|GetDialogueWidget))
    (Variables|Default|SetEndDialogue false)
    (Variables|Default|SetDialogueWidget 0)
    (Components|Activation|Deactivate _sphere)
    (Variables|/Script/Engine.PrimitiveComponent|SetbGenerateOverlapEvents _sphere false)
    (bind _asbp_player (Utilities|Casting|CastToBP_Player (Game|GetPlayerCharacter 0)))
    (Default|GoAway _asbp_player)
    (Game|Player|SetViewTargetwithBlend _returnvalue (Pawn|GetControlledPawn _returnvalue) 1.0 "VTBlend_Linear" 0.0 false)
    (Utilities|FlowControl|Delay 0.2)
    (Variables|/Game/BluePrints/BP_Player.BP_Player_C|SetPaused (Variables|Default|GetAs%20BP%20Player) false)
    (Variables|Default|SetCurrentlyInteractedWith 0)
    (else
      (Development|PrintString "it's valid")
      (bind _returnvalue_2 (Utilities|GetDataTableRow (Variables|Default|GetData%20Table) (Variables|Default|GetRow%20Name))
        (:then
          (Default|UpdateDialogue (Variables|Default|GetDialogueWidget) (.Dialogue (Utilities|Struct|BreakDialogue1 _returnvalue_2)))
          (Variables|Default|SetRow%20Name (.Row (Utilities|Struct|BreakDialogue1 _returnvalue_2)))
          (Variables|Default|SetData%20Table (.DataTable (Utilities|Struct|BreakDialogue1 _returnvalue_2)))
          (Variables|Default|SetEndDialogue (.EndDialogue (Utilities|Struct|BreakDialogue1 _returnvalue_2)))
          (Variables|Default|SetOpen%20Ended%20Dialogue? (.OpenEndedDialogue? (Utilities|Struct|BreakDialogue1 _returnvalue_2)))
          (Variables|Default|SetOpen%20Ended%20Dialogue%20Options (.OpenEndedDialogueOptions (Utilities|Struct|BreakDialogue1 _returnvalue_2)))
          (if (stale Collision|EventActorBeginOverlap _output_get_2)
            (for _array_element (stale Collision|EventActorBeginOverlap _output_get_3)
              (bind _returnvalue_3 (UserInterface|CreateWidget "/Game/WB_Option.WB_Option_C" 0 (Utilities|Text|ToText(Name) (.OptionName (Utilities|Struct|BreakOptionsDialogueStrucutre _array_element))) self (.Row (Utilities|Struct|BreakOptionsDialogueStrucutre _array_element)) (.DataTable (Utilities|Struct|BreakOptionsDialogueStrucutre _array_element))))
              (Widget|Panel|AddChild (Variables|/Game/DialogueWidget.DialogueWidget_C|GetOptionScrollBox (Variables|Default|GetDialogueWidget)) _returnvalue_3)
              (bind _output_get (Variables|Default|SetCurrentOption _returnvalue_3)))))))))

(event Custom|OptionSelected
  (params (DataTable :type Data%20Table%20Object%20Reference) (RowName :type Name))
  (bind _dialoguewidget (Variables|Default|GetDialogueWidget))
  (bind _returnvalue (Utilities|GetDataTableRow DataTable RowName)
    (:then
      (Default|UpdateDialogue _dialoguewidget (.Dialogue (Utilities|Struct|BreakDialogue1 _returnvalue)))
      (Variables|Default|SetRow%20Name (.Row (Utilities|Struct|BreakDialogue1 _returnvalue)))
      (Variables|Default|SetEndDialogue (.EndDialogue (Utilities|Struct|BreakDialogue1 _returnvalue)))
      (Variables|Default|SetData%20Table (.DataTable (Utilities|Struct|BreakDialogue1 _returnvalue)))
      (Widget|Panel|ClearChildren (Variables|/Game/DialogueWidget.DialogueWidget_C|GetOptionScrollBox _dialoguewidget)))))

(event EventBeginPlay
  (bind _sphere (Variables|Default|GetSphere))
  (Components|Activation|Deactivate _sphere)
  (Variables|/Script/Engine.PrimitiveComponent|SetbGenerateOverlapEvents _sphere false))

(event Collision|EventActorBeginOverlap
  (params (OtherActor :type Actor%20Object%20Reference))
  (bind _sphere (Variables|Default|GetSphere))
  (Components|Activation|Deactivate _sphere)
  (AI|Navigation|SimpleMovetoLocation (Game|GetPlayerController 0) (.location (Transformation|GetActorTransform (Game|GetPlayerCharacter 0))))
  (Variables|/Script/Engine.PrimitiveComponent|SetbGenerateOverlapEvents _sphere false)
  (Game|Player|SetViewTargetwithBlend (Game|GetPlayerController 0) self 1.0 "VTBlend_Linear" 0.0 false)
  (bind _asbp_player (Utilities|Casting|CastToBP_Player (Game|GetPlayerCharacter 0)))
  (bind _output_get (Variables|Default|SetAs%20BP%20Player _asbp_player))
  (Variables|/Game/BluePrints/BP_Player.BP_Player_C|SetPaused _output_get true)
  (Default|GoAway _output_get)
  (bind _returnvalue (Utilities|GetDataTableRow (Variables|Default|GetData%20Table) (Variables|Default|GetRow%20Name))
    (:then
      (bind _returnvalue_2 (UserInterface|CreateWidget "/Game/DialogueWidget.DialogueWidget_C" (Game|GetPlayerController 0) (Utilities|Text|ToText(String) (Utilities|GetDisplayName self)) (.Dialogue (Utilities|Struct|BreakDialogue1 _returnvalue))))
      (UserInterface|Viewport|AddtoPlayerScreen _returnvalue_2)
      (Variables|Default|SetDialogueWidget _returnvalue_2)
      (Variables|Default|SetRow%20Name (.Row (Utilities|Struct|BreakDialogue1 _returnvalue)))
      (Variables|Default|SetData%20Table (.DataTable (Utilities|Struct|BreakDialogue1 _returnvalue)))
      (Variables|Default|SetEndDialogue (.EndDialogue (Utilities|Struct|BreakDialogue1 _returnvalue)))
      (bind _output_get_2 (Variables|Default|SetOpen%20Ended%20Dialogue? (.OpenEndedDialogue? (Utilities|Struct|BreakDialogue1 _returnvalue))))
      (bind _output_get_3 (Variables|Default|SetOpen%20Ended%20Dialogue%20Options (.OpenEndedDialogueOptions (Utilities|Struct|BreakDialogue1 _returnvalue))))
      (if _output_get_2
        (for _array_element _output_get_3
          (bind _returnvalue_3 (UserInterface|CreateWidget "/Game/WB_Option.WB_Option_C" 0 (Utilities|Text|ToText(Name) (.OptionName (Utilities|Struct|BreakOptionsDialogueStrucutre _array_element))) self (.Row (Utilities|Struct|BreakOptionsDialogueStrucutre _array_element)) (.DataTable (Utilities|Struct|BreakOptionsDialogueStrucutre _array_element))))
          (Widget|Panel|AddChild (Variables|/Game/DialogueWidget.DialogueWidget_C|GetOptionScrollBox (Variables|Default|GetDialogueWidget)) _returnvalue_3)
          (bind _output_get_4 (Variables|Default|SetCurrentOption _returnvalue_3)))))))

(event EventInspect
  (bind _returnvalue (Game|AddComponentbyClass "/Script/UMG.WidgetComponent" false (Math|Transform|MakeTransform "0.000000,0.000000,100.000000" "0, 0, 0" "1.000000,1.000000,1.000000")))
  (Variables|Default|SetAddedWidget _returnvalue)
  (bind _returnvalue_2 (UserInterface|CreateWidget "/Game/InspectText.InspectText_C" 0 (Variables|Default|GetInspect%20Text)))
  (bind _output_get (Variables|Default|SetInspectTextReference _returnvalue_2))
  (UserInterface|SetWidget (Variables|Default|GetAddedWidget) _output_get)
  (Collision|SetCollisionEnabled (Variables|Default|GetAddedWidget) "NoCollision")
  (Class|WidgetComponent|SetWidgetSpace (Variables|Default|GetAddedWidget) "Screen")
  (Transformation|SetRelativeLocation (Variables|Default|GetAddedWidget) "0.000000,0.000000,100.000000" false false)
  (Rendering|SetVisibility (Variables|Default|GetAddedWidget) true true)
  (Default|UpdateInspectText (Variables|Default|GetInspectTextReference) (Variables|Default|GetInspect%20Text))
  (Development|PrintString "Hello2")
  (Variables|Default|SetCurrentlyInteractedWith 0)
  (Utilities|FlowControl|Delay 3.0)
  (Rendering|SetVisibility (Variables|Default|GetAddedWidget) false false)
  (Components|DestroyComponent (Variables|Default|GetAddedWidget)))

(event EventInteract
  (params (PlayerRef :type BP%20Player%20Object%20Reference))
  (bind _asbp_player (Utilities|Casting|CastToBP_Player (Game|GetPlayerCharacter 0)))
  (Variables|/Game/ContextMenu.ContextMenu_C|SetIsWalkButtonVisible (Variables|/Game/MainHUd.MainHUd_C|GetContextMenu (Variables|/Game/BluePrints/BP_Player.BP_Player_C|GetMainHudRef _asbp_player)) true)
  (bind _output_get (Variables|/Game/ContextMenu.ContextMenu_C|SetIsInteractVisible (Variables|/Game/MainHUd.MainHUd_C|GetContextMenu (Variables|/Game/BluePrints/BP_Player.BP_Player_C|GetMainHudRef _asbp_player)) true))
  (Development|PrintString (Utilities|String|ToString(Boolean) _output_get))
  (EventDispatchers|BindEventtoWalkEvent (Variables|/Game/MainHUd.MainHUd_C|GetContextMenu (Variables|/Game/BluePrints/BP_Player.BP_Player_C|GetMainHudRef _asbp_player)) (delegate Custom|Talk))
  (bind _asbp_player_2 (Utilities|Casting|CastToBP_Player (Game|GetPlayerCharacter 0)))
  (bind _output_get_2 (Variables|/Game/MainHUd.MainHUd_C|SetCurrentlyInteractedWith (Variables|/Game/BluePrints/BP_Player.BP_Player_C|GetMainHudRef _asbp_player_2) (Variables|/Game/BluePrints/BP_Player.BP_Player_C|GetHit%20Actor _asbp_player_2)))
  (Development|PrintString (Utilities|GetDisplayName _output_get_2)))

(fn ConstructionScript)