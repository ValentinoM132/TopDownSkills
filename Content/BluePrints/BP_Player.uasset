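; Player character for a turn-based game with click-to-move, right-drag camera rotation, wheel zoom and an interact context menu.
; Cursor traces drive free-roam movement or, in restricted mode, range-limited walking and one Tentacles, Tidal Wave or Fireball cast per turn.
; Tick updates distance travelled, targeting cursor validity and the wave preview.
; StartTurn loops on a delay to spend walking range; Space ends the turn through BP_TurnBased.
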(event Custom|GoAway
  ;[0.15 0.15 0.15 0.5] GoAway (Go Invisible Event)
  (Utilities|FlowControl|FlipFlop
    (:A
      (Rendering|SetVisibility (Variables|Default|GetSKM_Manny_Simple) false false))
    (:B
      (Rendering|SetVisibility (Variables|Default|GetSKM_Manny_Simple) true false))))

(event Custom|EndingPlayerTurn
  ;[0.15 0.15 0.15 0.5] EndTurn on space
  (if (Class|KismetMathLibrary|XORBoolean (Variables|Default|GetTurnStarted) (Variables|Default|GetEndedTurn))
    (Variables|Default|SetRoundedRangeLeft 0)
    (bind _asbp_turn_based (Utilities|Casting|CastToBP_TurnBased (Game|GetGameMode)))
    (Default|EndTurn _asbp_turn_based)
    (Variables|Default|SetRangeLeft 1.5e+02)
    (Variables|Default|SetDummyTestFloat 0.0)
    (Variables|Default|SetAbilityExhausted false)
    (Variables|Default|SetTurnStarted false)
    (Variables|Default|SetEndedTurn true)
    (bind _asbp_turn_based_2 (Utilities|Casting|CastToBP_TurnBased (Game|GetGameMode)))
    (bind _output_get (Variables|Default|SetCount%20Down%20Timer (Variables|/Game/BluePrints/BP_TurnBased.BP_TurnBased_C|GetCountDownTimer _asbp_turn_based_2)))
    (Variables|Default|SetRoundsLeftString (Utilities|String|Append "Rounds Remaining 
Until Next Wave: " (Utilities|String|ToString(Integer) _output_get)))))

(event Input|EnhancedActionEvents|EnhancedInputActionIA_RightClick
  (params (ActionValue :type Boolean) (ElapsedSeconds :type Float%20%28double-precision%29) (TriggeredSeconds :type Float%20%28double-precision%29) (InputAction :type Input%20Action%20Object%20Reference :default "/Game/InputAction/IA_RightClick.IA_RightClick"))
  (bind _returnvalue (Game|GetPlayerController 0))
  (bind (_locationx _locationy) (Game|Player|GetMousePosition _returnvalue))
  ;[0.15 0.15 0.15 0.5] RightClick
  (:Triggered
    (Variables|/Script/Engine.PlayerController|SetbShowMouseCursor (Game|GetPlayerController 0) false :!label _label)
    (Variables|Default|SetRightClickHeld true)
    (Input|SetInputModeGameOnly (Game|GetPlayerController 0) false)
    (if (Variables|Default|GetInContextMenu)
      (Default|CloseContext (Variables|Default|GetMainHudRef))
      (Utilities|FlowControl|Delay 0.2)
      (Variables|Default|SetInContextMenu false)))
  (:Started
    (Variables|Default|SetMousePositionX _locationx)
    (Variables|Default|SetMousePositionY _locationy))
  (:Ongoing
    (goto _label))
  (:Completed
    (Variables|/Script/Engine.PlayerController|SetbShowMouseCursor (Game|GetPlayerController 0) true)
    (Variables|Default|SetRightClickHeld false)
    (Class|PlayerController|SetMouseLocation (Game|GetPlayerController 0) (Math|Float|Truncate (Variables|Default|GetMousePositionX)) (Math|Float|Truncate (Variables|Default|GetMousePositionY)))
    (Input|SetInputModeGameandUI (Game|GetPlayerController 0) 0 "LockAlways" false false)))

(event Input|EnhancedActionEvents|EnhancedInputActionIA_LeftClick
  (params (ActionValue :type Boolean) (ElapsedSeconds :type Float%20%28double-precision%29) (TriggeredSeconds :type Float%20%28double-precision%29) (InputAction :type Input%20Action%20Object%20Reference :default "/Game/InputAction/IA_LeftClick.IA_LeftClick"))
  (bind _returnvalue (Game|GetPlayerController 0))
  (bind _returnvalue_2 (Game|GetPlayerController 0))
  (bind _returnvalue_3 (Game|GetPlayerController 0))
  (bind _returnvalue_4 (Game|Player|GetPlayerPawn 0))
  (bind _returnvalue_5 (Game|GetPlayerCharacter 0))
  (bind (_worldlocation _worlddirection) (Game|Player|ConvertMouseLocationToWorldSpace _returnvalue))
  (bind (_worldlocation_2 _worlddirection_2) (Game|Player|ConvertMouseLocationToWorldSpace _returnvalue_2))
  (bind (_worldlocation_3 _worlddirection_3) (Game|Player|ConvertMouseLocationToWorldSpace _returnvalue_3))
  (bind _returnvalue_6 (Transformation|GetVelocity _returnvalue_4))
  (bind _returnvalue_7 (Transformation|GetActorTransform _returnvalue_5))
  (bind _returnvalue_8 (Math|Vector|VectorLength _returnvalue_6))
  (bind _returnvalue_9 (<= _returnvalue_8 0.0))
  ;[0.15 0.15 0.15 0.5] Left Click + Movement
  (:Triggered
    (if (Variables|Default|GetPaused) :!label _label
      (if (not (Variables|Default|GetHasClicked))
        (bind _asbp_npc (Utilities|Casting|CastToBP_NPC (Variables|Default|GetHit%20Actor)))
        (Default|MouseClicked _asbp_npc)
        (Variables|Default|SetHasClicked true)
        (Utilities|FlowControl|Delay 0.2)
        (Variables|Default|SetHasClicked false))
      (else
        (switch Utilities|FlowControl|Switch|SwitchonPlayerMovementState (Variables|Default|GetCurrentMovementState)
          (:NewEnumerator0
            (bind (_outhit _returnvalue_10) (Collision|LineTraceByChannel _worldlocation_3 (+ _worldlocation_3 (* _worlddirection_3 1e+04)) "TraceTypeQuery1" false 0 "None" :!label _label_2))
            (if _returnvalue_10
              (if (not (Utilities|DoesObjectImplementInterface (.HitActor (Collision|BreakHitResult _outhit)) "/Game/BluePrints/BPI_Interact.BPI_Interact_C"))
                (AI|Navigation|SimpleMovetoLocation (Pawn|GetController) (.Location (Collision|BreakHitResult _outhit)))
                (Default|CloseContext (Variables|Default|GetMainHudRef)))))
          (:NewEnumerator1
            (switch Utilities|FlowControl|Switch|SwitchonCurrentSelectedAbility (Variables|Default|GetCurrentState)
              (:NewEnumerator0
                (if (Variables|Default|GetTurnStarted)
                  (if (Class|KismetMathLibrary|XORBoolean (Variables|Default|GetRangeEquals0) (Variables|Default|GetTurnStarted))
                    (Variables|Default|SetIsMoving _returnvalue_9)
                    (if _returnvalue_9
                      (if (not (Variables|Default|GetEndedTurn))
                        (Variables|Default|SetstartingLocation (Transformation|GetActorLocation))
                        (goto _label_2))))))
              (:NewEnumerator1
                (if (Variables|Default|Get!HadarValid)
                  (Development|PrintString "Too Far, Try closer")
                  (elif (not (Variables|Default|GetAbilityExhausted))
                    (bind (_outhit_2 _returnvalue_11) (Collision|LineTraceByChannel _worldlocation (+ _worldlocation (* _worlddirection 1e+04)) "TraceTypeQuery1" false 0 "None"))
                    (if _returnvalue_11
                      (bind _returnvalue_12 (Game|SpawnActorfromClass "/Game/Tentacle.Tentacle_C" (Math|Transform|MakeTransform (.Location (Collision|BreakHitResult _outhit_2)) "0, 0, 0" "1.000000,1.000000,1.000000") "AlwaysSpawn" "MultiplyWithRoot" 0 0))
                      (Variables|Default|SetAbilityExhausted true)
                      (Utilities|FlowControl|Delay 2.0)
                      (Actor|DestroyActor _returnvalue_12)
                      (Default|HadarColorChange (Variables|Default|GetMainHudRef))))))
              (:NewEnumerator2
                (if (not (Variables|Default|GetAbilityExhausted))
                  (Game|SpawnActorfromClass "/Game/BP_TidalWave.BP_TidalWave_C" (Math|Transform|MakeTransform (Math|Vector|MakeVector (.x (.location _returnvalue_7)) (.y (.location _returnvalue_7)) (- (.z (.location _returnvalue_7)) 6e+01)) (.rotation _returnvalue_7) (.scale _returnvalue_7)) "Undefined" "MultiplyWithRoot" 0 0)
                  (Actor|DestroyActor (Variables|Default|GetTidalWaveArea))
                  (Variables|Default|SetAbilityExhausted true)
                  (Utilities|FlowControl|Delay 0.2)
                  (Default|TidalWaveColorChange (Variables|Default|GetMainHudRef))
                  (Variables|Default|SetFlipperOut false)))
              (:NewEnumerator3
                (if (Variables|Default|Get!Fireball%20Valid)
                  (Development|PrintString "Too Far, Try closer")
                  (else
                    (Variables|Default|SetIsAiming false)
                    (if (not (Variables|Default|GetAbilityExhausted))
                      (bind _returnvalue_13 (Game|SpawnActorfromClass "/Game/BluePrints/Fireball.Fireball_C" (Math|Transform|MakeTransform (Transformation|GetWorldLocation (Variables|Default|GetGrenadeRef)) (Transformation|GetActorRotation) "1.000000,1.000000,1.000000") "Undefined" "MultiplyWithRoot" 0 "0.000000,0.000000,200.000000" 1.0 0))
                      (bind _outhit_3 (Collision|LineTraceByChannel _worldlocation_2 (+ _worldlocation_2 (* _worlddirection_2 1e+04)) "TraceTypeQuery1" false 0 "Persistent"))
                      (bind (_outlaunchvelocity _returnvalue_14) (Game|SuggestProjectileVelocityCustomArc (Transformation|GetActorLocation _returnvalue_13) (.location _outhit_3) 0.0 0.5))
                      (if _returnvalue_14
                        (Physics|SetPhysicsLinearVelocity (Variables|/Game/BluePrints/Fireball.Fireball_C|GetFireballBall _returnvalue_13) _outlaunchvelocity false "None")
                        (Variables|Default|SetAbilityExhausted true)
                        (Utilities|FlowControl|Delay 0.2)
                        (Default|FireballColorChange (Variables|Default|GetMainHudRef)))))))))))))
  (:Ongoing
    (goto _label)))

(event Input|EnhancedActionEvents|EnhancedInputActionIA_MouseX
  (params (ActionValue :type Float%20%28double-precision%29) (ElapsedSeconds :type Float%20%28double-precision%29) (TriggeredSeconds :type Float%20%28double-precision%29) (InputAction :type Input%20Action%20Object%20Reference :default "/Game/InputAction/IA_MouseX.IA_MouseX"))
  ;[0.15 0.15 0.15 0.5] Rotates Camera while right click is held
  (:Triggered
    (if (Variables|Default|GetRightClickHeld) :!label _label
      (Pawn|Input|AddControllerYawInput ActionValue)))
  (:Ongoing
    (goto _label)))

(event Input|EnhancedActionEvents|EnhancedInputActionIA_RightClickTap
  (params (ActionValue :type Boolean) (ElapsedSeconds :type Float%20%28double-precision%29) (TriggeredSeconds :type Float%20%28double-precision%29) (InputAction :type Input%20Action%20Object%20Reference :default "/Game/InputAction/IA_RightClickTap.IA_RightClickTap"))
  (bind _returnvalue (Game|GetPlayerController 0))
  (bind _returnvalue_2 (Game|GetPlayerController 0))
  (bind (_worldlocation _worlddirection) (Game|Player|ConvertMouseLocationToWorldSpace _returnvalue))
  (bind (_locationx _locationy) (Game|Player|GetMousePosition _returnvalue_2))
  ;[0.15 0.15 0.15 0.5] Check if interactable has been right clicked
  (:Started
    (bind _outhit (Collision|LineTraceByChannel _worldlocation (+ _worldlocation (* _worlddirection 1e+04)) "TraceTypeQuery1" false 0 "None"))
    (if (Utilities|DoesObjectImplementInterface (.HitActor (Collision|BreakHitResult _outhit)) "/Game/BluePrints/BPI_Interact.BPI_Interact_C")
      (bind _output_get (Variables|Default|SetHit%20Actor (.HitActor (Collision|BreakHitResult _outhit))))
      (Class|BPIInteract|Interact(Message) _output_get)
      (Variables|Default|SetMousePos (Math|Vector|MakeVector _locationx _locationy 0.0))
      (Default|OpenContext (Variables|Default|GetMainHudRef))
      (Utilities|FlowControl|Delay 0.2)
      (Variables|Default|SetInContextMenu true))))

(event EventStartTurn
  ;[0.15 0.15 0.15 0.5] Range Calculations
  (bind _asbp_turn_based (Utilities|Casting|CastToBP_TurnBased (Game|GetGameMode)))
  (bind _output_get (Variables|Default|SetCount%20Down%20Timer (Variables|/Game/BluePrints/BP_TurnBased.BP_TurnBased_C|GetCountDownTimer _asbp_turn_based)))
  (Variables|Default|SetRoundsLeftString (Utilities|String|Append "Rounds Remaining 
Until Next Wave: " (Utilities|String|ToString(Integer) _output_get)))
  (Variables|Default|SetTurnStarted true)
  (Variables|Default|SetRangeEquals0 false)
  (Variables|Default|SetEndedTurn false)
  (bind _output_get_2 (Variables|Default|SetDummyTestFloat (- (Variables|Default|GetDummyTestFloat) (Variables|Default|GetDistanceTravelled))))
  (bind _output_get_3 (Variables|Default|SetRoundedRangeLeft (Math|Float|Round (+ _output_get_2 (Variables|Default|GetRangeLeft)))))
  (bind _output_get_4 (Variables|Default|SetRangeDividedby5 (/ _output_get_3 5)))
  (Utilities|FlowControl|Delay 0.1)
  (Variables|Default|SetSpeedString (Utilities|String|Append "Walking Range = " (Utilities|String|ToString(Integer) (Math|Integer|Clamp(Integer) _output_get_4 0 30))))
  (if (<= (Variables|Default|GetRoundedRangeLeft) 0)
    (Components|Movement|StopMovementImmediately (Variables|Character|GetCharacterMovement))
    (Variables|Default|SetRangeEquals0 true)
    (else
      (CallFunction|StartTurn))))

(event EventTick
  (params (DeltaSeconds :type Float%20%28single-precision%29))
  (bind _returnvalue (Transformation|GetActorTransform))
  (bind _returnvalue_2 (Game|GetPlayerController 0))
  (bind _returnvalue_3 (Game|GetPlayerController 0))
  (bind _returnvalue_4 (Transformation|GetActorLocation))
  (bind (_worldlocation _worlddirection) (Game|Player|ConvertMouseLocationToWorldSpace _returnvalue_2))
  (bind (_worldlocation_2 _worlddirection_2) (Game|Player|ConvertMouseLocationToWorldSpace _returnvalue_3))
  (switch Utilities|FlowControl|Switch|SwitchonCurrentSelectedAbility (Variables|Default|GetCurrentState)
    (:NewEnumerator0
      (Class|PlayerController|SetMouseCursorWidget (Game|GetPlayerController 0) "Default" (Variables|Default|GetCursor%20Normal))
      (Utilities|IsValid (Variables|Default|GetTidalWaveArea)
        (:Is%20Valid
          ;[0.15 0.15 0.15 0.5] Void update() using to calculate distance traveled
          (Actor|DestroyActor (Variables|Default|GetTidalWaveArea))
          (Variables|Default|SetFlipperOut false))
        (:Is%20Not%20Valid
          _))
      (if (Variables|Default|GetTurnStarted)
        (bind _output_get (Variables|Default|SetCurrentLocation (Transformation|GetActorLocation)))
        (Variables|Default|SetDistanceTravelled (Math|Vector|Distance(Vector) _output_get (Variables|Default|GetstartingLocation)))
        (Variables|Default|SetstartingLocation (Transformation|GetActorLocation))))
    (:NewEnumerator1
      (if (Variables|Default|Get!HadarValid)
        (Variables|/Game/BluePrints/WBP_CustomCursor.WBP_CustomCursor_C|SetIsGreen (Variables|Default|GetWBP%20Custom%20Cursor) false)
        (else
          (Variables|/Game/BluePrints/WBP_CustomCursor.WBP_CustomCursor_C|SetIsGreen (Variables|Default|GetWBP%20Custom%20Cursor) true)))
      (Class|PlayerController|SetMouseCursorWidget (Game|GetPlayerController 0) "Default" (Variables|Default|GetWBP%20Custom%20Cursor) :!label _label)
      (bind _outhit (Collision|LineTraceByChannel _worldlocation_2 (+ _worldlocation_2 (* _worlddirection_2 1e+04)) "TraceTypeQuery1" false 0 "None"))
      (Variables|Default|SetMouseDistanceFromPlayer (Math|Vector|Distance(Vector) (.location _outhit) (Transformation|GetActorLocation)))
      (Variables|Default|Set!Fireball%20Valid (>= (Variables|Default|GetMouseDistanceFromPlayer) (Variables|Default|GetFireballRange)))
      (Variables|Default|Set!HadarValid (>= (Variables|Default|GetMouseDistanceFromPlayer) (Variables|Default|GetHadarRange))))
    (:NewEnumerator2
      (if (not (Variables|Default|GetAbilityExhausted))
        (Transformation|SetActorRotation (Math|Rotator|MakeRotator 0.0 0.0 (.yaw (Math|Rotator|FindLookatRotation _returnvalue_4 (.Intersection (Class|KismetMathLibrary|LinePlaneIntersectionOriginNormal _worldlocation (+ _worldlocation (* _worlddirection 1e+04)) _returnvalue_4 "0.000000,0.000000,1.000000"))))))
        (if (not (Variables|Default|GetFlipperOut))
          (bind _returnvalue_5 (Game|SpawnActorfromClass "/Game/BP_TidalWaveArea.BP_TidalWaveArea_C" (Math|Transform|MakeTransform (Math|Vector|MakeVector (.x (.location _returnvalue)) (.y (.location _returnvalue)) (- (.z (.location _returnvalue)) 3e+02)) (.rotation _returnvalue) (.scale _returnvalue)) "AlwaysSpawn" "MultiplyWithRoot" self 0))
          (bind _output_get_2 (Variables|Default|SetTidalWaveArea _returnvalue_5))
          (Variables|Default|SetFlipperOut true)
          (Transformation|AttachComponentToComponent _output_get_2 (Variables|Collision|GetCapsuleComponent) "None" "SnapToTarget" "SnapToTarget" "SnapToTarget" true))))
    (:NewEnumerator3
      (if (Variables|Default|Get!Fireball%20Valid)
        (Variables|/Game/BluePrints/WBP_CustomCursor.WBP_CustomCursor_C|SetIsGreen (Variables|Default|GetWBP%20Custom%20Cursor) false)
        (goto _label)
        (else
          (Variables|/Game/BluePrints/WBP_CustomCursor.WBP_CustomCursor_C|SetIsGreen (Variables|Default|GetWBP%20Custom%20Cursor) true)
          (goto _label))))))

(event EventBeginPlay
  ;[0.15 0.15 0.15 0.5] EventBeginPlay (ShowCursor,AddMainHud,SetStartingLocation)
  (Variables|/Script/Engine.PlayerController|SetbShowMouseCursor (Game|GetPlayerController 0) true)
  (bind _returnvalue (UserInterface|CreateWidget "/Game/MainHUd.MainHUd_C"))
  (bind _output_get (Variables|Default|SetMainHudRef _returnvalue))
  (UserInterface|Viewport|AddtoViewport _output_get 0)
  (Variables|Default|SetstartingLocation (Transformation|GetActorLocation))
  (Variables|Default|SetWBP%20Custom%20Cursor (Variables|/Game/MainHUd.MainHUd_C|GetWBP_CustomCursor (Variables|Default|GetMainHudRef)))
  (Variables|Default|SetCursor%20Normal (Variables|/Game/MainHUd.MainHUd_C|GetCursorNormal (Variables|Default|GetMainHudRef)))
  (bind _asbp_turn_based (Utilities|Casting|CastToBP_TurnBased (Game|GetGameMode)))
  (bind _output_get_2 (Variables|Default|SetCount%20Down%20Timer (Variables|/Game/BluePrints/BP_TurnBased.BP_TurnBased_C|GetCountDownTimer _asbp_turn_based)))
  (Variables|Default|SetRoundsLeftString (Utilities|String|Append "Rounds Remaining 
Until Next Wave: " (Utilities|String|ToString(Integer) _output_get_2))))

(event Input|MouseEvents|MouseWheelAxis
  (params (AxisValue :type Float%20%28single-precision%29))
  ;[0.15 0.15 0.15 0.5] Zoom In and Out
  (bind _output_get (Variables|Default|SetSpringArm (Variables|Default|GetSpringArm)))
  (bind _output_get_2 (Variables|Default|SetCameraOffset+Length (Math|Float|Clamp(Float) (+ (* AxisValue -1e+02) (Variables|Default|GetCameraOffset+Length)) 2e+02 5e+02)))
  (Variables|/Script/Engine.SpringArmComponent|SetTargetArmLength _output_get _output_get_2)
  (Variables|/Script/Engine.SpringArmComponent|SetTargetOffset _output_get (Math|Vector|MakeVector 0.0 0.0 _output_get_2)))

(event Input|KeyboardEvents|SpaceBar
  (params (Key :type Key%20Structure :default "None"))
  ;[0.15 0.15 0.15 0.5] EndTurn on space
  (:Pressed
    (CallFunction|EndingPlayerTurn)))

(fn ConstructionScript)

(fn OnRepIsMoving)