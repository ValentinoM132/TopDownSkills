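; BP_TurnBased runs a wave-based, turn-based battle between the player and spawned enemies.
; Each wave spawns its DT_WaveData count at random SpawnLocations, then queues all BPI_StartTurn actors with the player first.
; EndTurn advances the queue, messaging each actor and blending the camera to it.
; After a countdown of full rounds, or with one actor queued, the next wave starts; the missing-row handler EndWaveGame is empty.
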(event Custom|StartTurnBasedGame
  (bind _returnvalue (Game|GetPlayerCharacter 0))
  (CallFunction|StartWave)
  (if (Variables|Default|GetBattleMode)
    _
    (else
      (bind _asbp_player (Utilities|Casting|CastToBP_Player (Game|GetPlayerCharacter 0)))
      (Default|BattleUIToggle (Variables|/Game/BluePrints/BP_Player.BP_Player_C|GetMainHudRef _asbp_player))))
  (bind _outactors (Actor|GetAllActorswithInterface "/Game/BluePrints/BPI_StartTurn.BPI_StartTurn_C"))
  (bind _output_get (Variables|Default|SetOut%20Actors _outactors))
  (Utilities|Array|RemoveIndex _output_get (Utilities|Array|FindItem _output_get (Game|GetPlayerCharacter 0)))
  (Utilities|Array|Insert _output_get _returnvalue)
  (CallFunction|ProccessNextTurn (Variables|Default|GetCurrentInt))
  (Variables|Default|SetBattleMode true)
  (bind _asbp_player_2 (Utilities|Casting|CastToBP_Player _returnvalue))
  (Variables|/Game/BluePrints/BP_Player.BP_Player_C|SetCurrentMovementState _asbp_player_2 "NewEnumerator1"))

(event Custom|ProccessNextTurn
  (params (Current :type Integer))
  (bind _out_actors (Variables|Default|GetOut%20Actors))
  (bind _output (Utilities|Array|Get(acopy) _out_actors Current))
  (Class|BPIStartTurn|StartTurn(Message) _output)
  (Game|Player|SetViewTargetwithBlend (Game|GetPlayerController 0) _output 1.0 "VTBlend_Cubic" 0.0 false))

(event Custom|EndTurn
  (bind _output_get (Variables|Default|SetCurrentInt (+ (Variables|Default|GetCurrentInt) 1)))
  (if (> (Utilities|Array|Length (Variables|Default|GetOut%20Actors)) _output_get)
    (CallFunction|ProccessNextTurn _output_get)
    (else
      (Variables|Default|SetCurrentInt 0)
      (CallFunction|ProccessNextTurn)
      (Variables|Default|SetCountDownTimer (- (Variables|Default|GetCountDownTimer) 1))
      (if (or (== (Variables|Default|GetCountDownTimer) 0) (== (Utilities|Array|Length (Variables|Default|GetOut%20Actors)) 1))
        (Development|PrintString "RoundOver")
        (Math|Integer|IncrementInt (Variables|Default|GetCurrentWave)
          (:%20%20
            (CallFunction|StartTurnBasedGame)
            (Variables|Default|SetCountDownTimer 3)))))))

(event Custom|SpawnRandomEnemy)

(event Custom|StartWave
  (bind _returnvalue (Utilities|GetDataTableRow "/Game/BluePrints/DT_WaveData.DT_WaveData" (Utilities|String|StringToName (Utilities|String|ToString(Integer) (Variables|Default|GetCurrentWave))))
    (:then
      (for _index (range 1 (.amounttospawn _returnvalue))
        (bind _outactors (Actor|GetAllActorsOfClass "/Game/BluePrints/SpawnLocation.SpawnLocation_C"))
        (Default|SpawnEnemy (.OutItem (Utilities|Array|Random _outactors)))))
    (:RowNotFound
      (CallFunction|EndWaveGame))))

(event Custom|EndWaveGame)

(event EventBeginPlay)

(event EventTick
  (params (DeltaSeconds :type Float%20%28single-precision%29)))

(fn ConstructionScript)