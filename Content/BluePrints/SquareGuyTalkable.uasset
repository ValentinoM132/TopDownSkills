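; SquareGuyTalkable is an interactable NPC that can be inspected and can start a turn-based game.
; Interact switches the player HUD's context menu from walk to interact options and registers this actor as the interaction target.
; Inspect spawns a temporary screen-space text widget above the actor and destroys it after a delay.
; InteractUpon calls StartTurnBasedGame on the BP_TurnBased game mode.
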(event EventBeginPlay)

(event Collision|EventActorBeginOverlap
  (params (OtherActor :type Actor%20Object%20Reference)))

(event EventInteractUpon
  (bind _asbp_turn_based (Utilities|Casting|CastToBP_TurnBased (Game|GetGameMode)))
  (Default|StartTurnBasedGame _asbp_turn_based))

(event EventInspect
  (bind _returnvalue (Game|AddComponentbyClass "/Script/UMG.WidgetComponent" false (Math|Transform|MakeTransform "0.000000,0.000000,100.000000" "0, 0, 0" "1.000000,1.000000,1.000000")))
  (Variables|Default|SetAddedWidget _returnvalue)
  (bind _returnvalue_2 (UserInterface|CreateWidget "/Game/InspectText.InspectText_C" 0 (Utilities|Text|FormatText (Variables|Default|GetInspect%20Text) (Utilities|Text|MakeLiteralText " 
"))))
  (bind _output_get (Variables|Default|SetInspectTextReference _returnvalue_2))
  (UserInterface|SetWidget (Variables|Default|GetAddedWidget) _output_get)
  (Collision|SetCollisionEnabled (Variables|Default|GetAddedWidget) "NoCollision")
  (Class|WidgetComponent|SetWidgetSpace (Variables|Default|GetAddedWidget) "Screen")
  (Transformation|SetRelativeLocation (Variables|Default|GetAddedWidget) "0.000000,0.000000,100.000000" false false)
  (Rendering|SetVisibility (Variables|Default|GetAddedWidget) true true)
  (Default|UpdateInspectText (Variables|Default|GetInspectTextReference) (Utilities|Text|FormatText (Variables|Default|GetInspect%20Text) (Utilities|Text|MakeLiteralText " 
")))
  (Utilities|FlowControl|Delay (Variables|Default|GetTextLengthDelay))
  (Rendering|SetVisibility (Variables|Default|GetAddedWidget) false false)
  (Components|DestroyComponent (Variables|Default|GetAddedWidget)))

(event EventInteract
  (params (PlayerRef :type BP%20Player%20Object%20Reference))
  (bind _asbp_player (Utilities|Casting|CastToBP_Player (Game|GetPlayerCharacter 0)))
  (Variables|/Game/ContextMenu.ContextMenu_C|SetIsWalkButtonVisible (Variables|/Game/MainHUd.MainHUd_C|GetContextMenu (Variables|/Game/BluePrints/BP_Player.BP_Player_C|GetMainHudRef _asbp_player)) false)
  (Variables|/Game/ContextMenu.ContextMenu_C|SetIsInteractVisible (Variables|/Game/MainHUd.MainHUd_C|GetContextMenu (Variables|/Game/BluePrints/BP_Player.BP_Player_C|GetMainHudRef _asbp_player)) true)
  (Variables|/Game/ContextMenu.ContextMenu_C|SetIsRealInteractVisible (Variables|/Game/MainHUd.MainHUd_C|GetContextMenu (Variables|/Game/BluePrints/BP_Player.BP_Player_C|GetMainHudRef _asbp_player)) true)
  (Variables|Default|SetCurrentlyInteractedWithRightNow self)
  (bind _asbp_player_2 (Utilities|Casting|CastToBP_Player (Game|GetPlayerCharacter 0)))
  (Variables|/Game/MainHUd.MainHUd_C|SetCurrentlyInteractedWith (Variables|/Game/BluePrints/BP_Player.BP_Player_C|GetMainHudRef _asbp_player_2) (Variables|Default|GetCurrentlyInteractedWithRightNow)))

(event EventTick
  (params (DeltaSeconds :type Float%20%28single-precision%29)))

(fn ConstructionScript)